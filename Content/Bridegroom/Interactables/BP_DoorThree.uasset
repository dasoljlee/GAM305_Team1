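; BP_DoorThree is an interactable door that rises for a player with a high enough score, then lowers itself.
; Interaction passes a score check and a DoOnce, then plays a world-move sound and raise timeline; after a delay, Lower repeats this downward and resets the gate.
; Both timelines lerp from the door's current location each update, so movement accumulates per tick rather than between fixed endpoints.
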(event `self.INT_Interact`
  (params (PlayerRef :type "/Game/Bridegroom/Blueprints/Player/PlayerCharacter_BP Object Reference") (Location :type "Vector Structure") (Hit :type "PrimitiveComponent Object Reference"))
  (bind _relativelocation (`SceneComponent.RelativeLocation` (`self.Door`)))
  ; Check Door
  (if (>= (`/Game/Bridegroom/Blueprints/Player/PlayerCharacter_BP.CurrentScore?` PlayerRef) 15.0)
    (`/Engine/EditorBlueprintResources/StandardMacros.DoOnce` false :!label _label
      (:`Completed`
        (`|ExecutionSequence`
          (:`then_0`
            (bind (_direction _newtrack_0) (`Timeline|Timeline` :!via `PlayFromStart`)
              (:`Update`
                (`SceneComponent.K2_SetRelativeLocation` (`self.Door`) (`KismetMathLibrary.VLerp` _relativelocation (+ _relativelocation (0.0 0.0 2.0)) _newtrack_0) false false))
              (:`Finished`
                (`KismetSystemLibrary.Delay` 5.0)
                (`self.Lower`))))
          (:`then_1`
            (`GameplayStatics.PlaySoundAtLocation` "/Engine/VREditor/Sounds/VR_WorldMoveLoop_01_Cue.VR_WorldMoveLoop_01_Cue" (`SceneComponent.K2_GetComponentLocation` (`self.Door`)) (struct) 1.0 1.0 0.0 "/Game/Bridegroom/Blueprints/Player/SoundAtten_BP.SoundAtten_BP" null null null)))))))

(event `Lower`
  (bind _relativelocation (`SceneComponent.RelativeLocation` (`self.Door`)))
  ; Check Door
  (`GameplayStatics.PlaySoundAtLocation` "/Engine/VREditor/Sounds/VR_WorldMoveLoop_01_Cue.VR_WorldMoveLoop_01_Cue" (`SceneComponent.K2_GetComponentLocation` (`self.Door`)) (struct) 1.0 1.0 0.0 "/Game/Bridegroom/Blueprints/Player/SoundAtten_BP.SoundAtten_BP" null null null)
  (bind (_direction _newtrack_0) (`Timeline|Timeline_0` :!via `PlayFromStart`)
    (:`Update`
      (`SceneComponent.K2_SetRelativeLocation` (`self.Door`) (`KismetMathLibrary.VLerp` _relativelocation (+ _relativelocation (0.0 0.0 -2.0)) _newtrack_0) false false))
    (:`Finished`
      (goto _label :!via `Reset`))))

(fn `UserConstructionScript`)