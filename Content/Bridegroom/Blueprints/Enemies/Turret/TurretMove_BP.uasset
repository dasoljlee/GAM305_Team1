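; Mobile turret enemy that chases the player and fires projectiles from its muzzle once alerted by detection overlap or damage.
; Looping timers drive pursuit and attacks; pursuit uses AI MoveTo toward a point beside the player, halting within stopping distance, while pivot and health widget face the player.
; Damage updates the health bar, flashes the body material and shows hitmarkers.
; Death plays a timeline scaling the pivot before destroying the actor.
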(event `self.ReceiveBeginPlay`
  ; Set Variables
  (`|ExecutionSequence`
    (:`then_0`
      (set `self.CurrentHealth` (`self.MaxHealth`)))
    (:`then_1`
      (`KismetMaterialLibrary.CreateDynamicMaterialInstance` "/Game/Bridegroom/Textures/FlashRed.FlashRed" "BodyColor")
      (`MeshComponent.SetVectorParameterValueOnMaterials` (`self.Body`) "BodyColor" (0.198 0.0569 0.137)))
    (:`then_2`
      (set `self.CanTakeDamage?` true))
    (:`then_3`
      (bind _asturret_w (cast `/Game/Bridegroom/Blueprints/Enemies/Turret/Turret_W` (`WidgetComponent.GetUserWidgetObject` (`self.Widget`))))
      (bind _output_get (set `self.As Turret W` _asturret_w))
      (`/Game/Bridegroom/Blueprints/Enemies/Turret/Turret_W.SetHealth` _output_get (`self.CurrentHealth`) (`self.MaxHealth`)))))

(event `self.ReceiveAnyDamage`
  (params (Damage :type "Float (single-precision)") (DamageType :type "DamageType Object Reference") (InstigatedBy :type "Controller Object Reference") (DamageCauser :type "Actor Object Reference"))
  ; Damage
  (if (`self.CanTakeDamage?`)
    (bind _asplayer_character_bp (cast `/Game/Bridegroom/Blueprints/Player/PlayerCharacter_BP` (`GameplayStatics.GetPlayerCharacter` 0)))
    (set `self.TargetPlayer` _asplayer_character_bp)
    (`self.Alert`)
    (`GameplayStatics.PlaySoundAtLocation` "/Engine/VREditor/Sounds/UI/Drop_Item_From_ContentBrowser.Drop_Item_From_ContentBrowser" (`SceneComponent.K2_GetComponentLocation` (`self.Body`)) (struct) 200.0 0.4 0.2 "/Game/Bridegroom/Blueprints/Player/SoundAtten_BP.SoundAtten_BP" null null null)
    (set `self.CurrentHealth` (- (`self.CurrentHealth`) Damage))
    (`/Game/Bridegroom/Blueprints/Enemies/Turret/Turret_W.SetHealth` (`self.As Turret W`) (`self.CurrentHealth`) (`self.MaxHealth`))
    (if (<= (`self.CurrentHealth`) 0.0)
      (`|ExecutionSequence`
        (:`then_1`
          (bind _returnvalue (`|CreateWidget` "/Game/Bridegroom/Blueprints/Player/Widgets/Hitmarker_W.Hitmarker_W_C"))
          (`UserWidget.AddToViewport` _returnvalue 0)
          (`/Game/Bridegroom/Blueprints/Player/Widgets/Hitmarker_W.HitAnim` _returnvalue)
          (set `self.CanTakeDamage?` false)
          (`self.DeadFlash`)
          (bind (_direction _newtrack_0) (`Timeline|Timeline_1`)
            (:`Update`
              (`SceneComponent.SetRelativeScale3D` (`self.Pivot`) (`KismetMathLibrary.Conv_DoubleToVector` _newtrack_0)))
            (:`Finished`
              (`GameplayStatics.PlaySoundAtLocation` "/Engine/VREditor/Sounds/VR_ungrab.VR_ungrab" (`self.K2_GetActorLocation` self) (struct) 0.5 1.0 0.2 "/Game/Bridegroom/Blueprints/Player/SoundAtten_BP.SoundAtten_BP" null null null)
              (`self.K2_DestroyActor`)
              (`KismetSystemLibrary.PrintString` "Hello")))))
      (else
        (`|ExecutionSequence`
          (:`then_0`
            (`self.Flash`))
          (:`then_1`
            (bind _returnvalue_2 (`|CreateWidget` "/Game/Bridegroom/Blueprints/Player/Widgets/Hitmarker_W.Hitmarker_W_C" null false))
            (`UserWidget.AddToViewport` _returnvalue_2 0)
            (`/Game/Bridegroom/Blueprints/Player/Widgets/Hitmarker_W.HitAnim` _returnvalue_2)))))))

(event `Alert`
  ; Detecting Player
  (`KismetSystemLibrary.K2_SetTimer` null "FollowPlayer" 0.05 true :!label _label)
  (set `self.IsDetected?` true)
  (`KismetSystemLibrary.K2_SetTimer` null "Attack Player" 1.2 true))

(event `self.Detection.OnComponentBeginOverlap`
  (params (OverlappedComponent :type "PrimitiveComponent Object Reference") (OtherActor :type "Actor Object Reference") (OtherComp :type "PrimitiveComponent Object Reference") (OtherBodyIndex :type Integer) (bFromSweep :type Boolean) (SweepResult :type "HitResult Structure (by ref)"))
  ; Detecting Player
  (bind _asplayer_character_bp (cast `/Game/Bridegroom/Blueprints/Player/PlayerCharacter_BP` OtherActor))
  (set `self.TargetPlayer` _asplayer_character_bp)
  (goto _label))

(event `self.Detection.OnComponentEndOverlap`
  (params (OverlappedComponent :type "PrimitiveComponent Object Reference") (OtherActor :type "Actor Object Reference") (OtherComp :type "PrimitiveComponent Object Reference") (OtherBodyIndex :type Integer))
  ; Detecting Player
  (cast `/Game/Bridegroom/Blueprints/Player/PlayerCharacter_BP` OtherActor)
  (`KismetSystemLibrary.K2_ClearTimer` null "FollowPlayer")
  (set `self.IsDetected?` false)
  (`KismetSystemLibrary.K2_ClearTimer` null "Attack Player"))

(event `DeadFlash`
  ; Death Flash
  (`MeshComponent.SetVectorParameterValueOnMaterials` (`self.Body`) "BodyColor" (1.0 0.0 0.0)))

(event `Flash`
  ; Flash Red When Taking Damage
  (`MeshComponent.SetVectorParameterValueOnMaterials` (`self.Body`) "BodyColor" (1.0 0.0 0.0))
  (`KismetSystemLibrary.Delay` 0.07)
  (`MeshComponent.SetVectorParameterValueOnMaterials` (`self.Body`) "BodyColor" (1.0 1.0 1.0))
  (`KismetSystemLibrary.Delay` 0.07)
  (`MeshComponent.SetVectorParameterValueOnMaterials` (`self.Body`) "BodyColor" (0.198 0.0569 0.137)))

(event `Attack Player`
  ; Attack Player
  (`GameplayStatics.PlaySoundAtLocation` "/Engine/VREditor/Sounds/UI/Scaling_Down.Scaling_Down" (`SceneComponent.K2_GetComponentLocation` (`self.Body`)) (struct) 2.0 1.5 0.0 "/Game/Bridegroom/Blueprints/Player/SoundAtten_BP.SoundAtten_BP" null null null)
  (`|SpawnActorFromClass` "/Game/Bridegroom/Blueprints/Enemies/Turret/TurretMoveProj_BP.TurretMoveProj_BP_C" (`SceneComponent.K2_GetComponentToWorld` (`self.Muzzle`)) "AlwaysSpawn" "MultiplyWithRoot" null null))

(event `FollowPlayer`
  (bind _returnvalue (`GameplayStatics.GetPlayerCharacter` 0))
  (bind _returnvalue_2 (`GameplayStatics.GetPlayerCharacter` 0))
  (bind _targetplayer (`self.TargetPlayer`))
  (bind _widget (`self.Widget`))
  (bind (_returnvalue_roll _returnvalue_pitch _returnvalue_yaw) (`KismetMathLibrary.BreakRotator` (`KismetMathLibrary.FindLookAtRotation` (`SceneComponent.K2_GetComponentLocation` _widget) (`self.K2_GetActorLocation` _returnvalue))))
  ; FollowPlayer
  (`|ExecutionSequence`
    (:`then_0`
      (`/Engine/EditorBlueprintResources/StandardMacros.IsValid` _targetplayer
        (:`Is Valid`
          (if (`self.IsDetected?`)
            (if (>= (`self.GetDistanceTo` _targetplayer) (`self.StoppingDistance`))
              (`|AIMoveTo` self (+ (`self.K2_GetActorLocation` (`self.TargetPlayer`)) (* (* (`self.OrbitSide`) (`SceneComponent.GetRightVector` (`/Game/Bridegroom/Blueprints/Player/PlayerCharacter_BP.Head` (`self.TargetPlayer`)))) 600.0)) null 300.0)
              (else
                (`MovementComponent.StopMovementImmediately` (`self.CharacterMovement`) :!label _label_2)))
            (else
              (goto _label_2))))))
    (:`then_1`
      (bind _asplayer_character_bp (cast `/Game/Bridegroom/Blueprints/Player/PlayerCharacter_BP` _returnvalue))
      (if (`/Game/Bridegroom/Blueprints/Player/PlayerCharacter_BP.IsPlayerAlive?` _asplayer_character_bp)
        (`SceneComponent.K2_SetWorldRotation` _widget (`KismetMathLibrary.MakeRotator` 0.0 0.0 _returnvalue_yaw) false false)))
    (:`then_2`
      (bind _asplayer_character_bp_2 (cast `/Game/Bridegroom/Blueprints/Player/PlayerCharacter_BP` _returnvalue_2))
      (if (`/Game/Bridegroom/Blueprints/Player/PlayerCharacter_BP.IsPlayerAlive?` _asplayer_character_bp_2)
        (`SceneComponent.K2_SetWorldRotation` (`self.Pivot`) (`KismetMathLibrary.FindLookAtRotation` (`self.K2_GetActorLocation`) (`self.K2_GetActorLocation` _returnvalue_2)) false false)))))

(fn `UserConstructionScript`)