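; Turret projectile actor that damages the player character on impact.
; The Projectile component's hit event casts the other actor to PlayerCharacter_BP and applies a small fixed damage to a valid player.
; It then destroys itself whether or not the player's CanTakeDamaage flag is set, and also on hitting anything else.
; The construction script sets a lifespan so stray shots expire.
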(event `self.Projectile.OnComponentHit`
  (params (HitComponent :type "PrimitiveComponent Object Reference") (OtherActor :type "Actor Object Reference") (OtherComp :type "PrimitiveComponent Object Reference") (NormalImpulse :type "Vector Structure") (Hit :type "HitResult Structure (by ref)"))
  ; Send Damage to Blob
  (bind _asplayer_character_bp (cast `/Game/Bridegroom/Blueprints/Player/PlayerCharacter_BP` OtherActor)
    (:`then`
      (`/Engine/EditorBlueprintResources/StandardMacros.IsValid` _asplayer_character_bp
        (:`Is Valid`
          (`GameplayStatics.ApplyDamage` _asplayer_character_bp 5.0 null self)
          (if (`/Game/Bridegroom/Blueprints/Player/PlayerCharacter_BP.CanTakeDamaage?` _asplayer_character_bp)
            (`self.K2_DestroyActor`)
            (else
              (`self.K2_DestroyActor`))))))
    (:`CastFailed`
      (`self.K2_DestroyActor`))))

(fn `UserConstructionScript`
  (`self.SetLifeSpan` 10.0))