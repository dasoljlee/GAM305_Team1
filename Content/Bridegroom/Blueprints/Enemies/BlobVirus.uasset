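; BlobVirus is an enemy that detects the player, approaches from a random side and attacks at close range.
; Detection overlaps toggle looping timers for facing and attacking, while Tick drives AI movement toward a side-offset point.
; Attacks launch the player, spin and stretch the pivot, then deal delayed damage, with DoOnce gates providing cooldown.
; Damage flashes the body material; death plays a scale timeline before destroying the actor.
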(event `self.ReceiveBeginPlay`
  ; Set Variables
  (`|ExecutionSequence`
    (:`then_0`
      (set `self.CurrentHealth` (`self.MaxHealth`)))
    (:`then_1`
      (`KismetMaterialLibrary.CreateDynamicMaterialInstance` "/Game/Bridegroom/Textures/FlashRed.FlashRed" "BodyColor")
      (`MeshComponent.SetVectorParameterValueOnMaterials` (`self.Body`) "BodyColor" (0.176 1.0 0.176)))
    (:`then_2`
      (set `self.OrbitSide` (`KismetMathLibrary.RandomFloatInRange` -1.0 1.0))
      (set `self.CanTakeDamage?` true))))

(event `self.ReceiveAnyDamage`
  (params (Damage :type "Float (single-precision)") (DamageType :type "DamageType Object Reference") (InstigatedBy :type "Controller Object Reference") (DamageCauser :type "Actor Object Reference"))
  ; Damage
  (if (`self.CanTakeDamage?`)
    (`GameplayStatics.PlaySoundAtLocation` "/Engine/VREditor/Sounds/UI/Drop_Item_From_ContentBrowser.Drop_Item_From_ContentBrowser" (`SceneComponent.K2_GetComponentLocation` (`self.Body`)) (struct) 300.0 0.4 0.2 null null null null)
    (bind _output_get (set `self.CurrentHealth` (- (`self.CurrentHealth`) Damage)))
    (if (<= _output_get 0.0)
      (set `self.CanTakeDamage?` false)
      (`self.DeadFlash`)
      (bind (_direction _newtrack_0) (`Timeline|Timeline_1` :!via `PlayFromStart`)
        (:`Update`
          (`SceneComponent.SetRelativeScale3D` (`self.Body`) (`KismetMathLibrary.Conv_DoubleToVector` _newtrack_0)))
        (:`Finished`
          (`GameplayStatics.PlaySoundAtLocation` "/Engine/VREditor/Sounds/VR_ungrab.VR_ungrab" (`self.K2_GetActorLocation` self) (struct) 1.0 1.0 0.2 null null null null)
          (`self.K2_DestroyActor`)))
      (else
        (`self.Flash`)))))

(event `FollowPlayer`
  (bind _returnvalue (`GameplayStatics.GetPlayerCharacter` 0))
  ; Follow Player With Rotation
  (bind _asplayer_character_bp (cast `/Game/Bridegroom/Blueprints/Player/PlayerCharacter_BP` _returnvalue))
  (if (`/Game/Bridegroom/Blueprints/Player/PlayerCharacter_BP.IsPlayerAlive?` _asplayer_character_bp)
    (`SceneComponent.K2_SetWorldRotation` (`self.Pivot`) (`KismetMathLibrary.FindLookAtRotation` (`self.K2_GetActorLocation`) (`self.K2_GetActorLocation` _returnvalue)) false false)))

(event `self.Detection.OnComponentBeginOverlap`
  (params (OverlappedComponent :type "PrimitiveComponent Object Reference") (OtherActor :type "Actor Object Reference") (OtherComp :type "PrimitiveComponent Object Reference") (OtherBodyIndex :type Integer) (bFromSweep :type Boolean) (SweepResult :type "HitResult Structure (by ref)"))
  ; Detecting Player
  (bind _asplayer_character_bp (cast `/Game/Bridegroom/Blueprints/Player/PlayerCharacter_BP` OtherActor))
  (set `self.TargetPlayer` _asplayer_character_bp)
  (`KismetSystemLibrary.K2_SetTimer` null "FollowPlayer" 0.05 true)
  (set `self.IsDetected?` true)
  (`KismetSystemLibrary.K2_SetTimer` null "Attack Player" 0.05 true))

(event `self.Detection.OnComponentEndOverlap`
  (params (OverlappedComponent :type "PrimitiveComponent Object Reference") (OtherActor :type "Actor Object Reference") (OtherComp :type "PrimitiveComponent Object Reference") (OtherBodyIndex :type Integer))
  ; Detecting Player
  (cast `/Game/Bridegroom/Blueprints/Player/PlayerCharacter_BP` OtherActor)
  (`KismetSystemLibrary.K2_ClearTimer` null "FollowPlayer")
  (set `self.IsDetected?` false)
  (`KismetSystemLibrary.K2_ClearTimer` null "Attack Player"))

(event `DeadFlash`
  ; Death Flash
  (`MeshComponent.SetVectorParameterValueOnMaterials` (`self.Body`) "BodyColor" (1.0 0.0 0.0)))

(event `Flash`
  ; Flash Red When Taking Damage
  (`MeshComponent.SetVectorParameterValueOnMaterials` (`self.Body`) "BodyColor" (1.0 0.0 0.0))
  (`KismetSystemLibrary.Delay` 0.07)
  (`MeshComponent.SetVectorParameterValueOnMaterials` (`self.Body`) "BodyColor" (1.0 1.0 1.0))
  (`KismetSystemLibrary.Delay` 0.07)
  (`MeshComponent.SetVectorParameterValueOnMaterials` (`self.Body`) "BodyColor" (0.176 1.0 0.176)))

(event `Attack Player`
  (bind _body (`self.Body`))
  (bind (_returnvalue_x _returnvalue_y) (`KismetMathLibrary.BreakVector` (* (`SceneComponent.GetForwardVector` _body) 600.0)))
  ; Attack Player
  (if (not (>= (`self.GetDistanceTo` (`self.TargetPlayer`)) (`self.StoppingDistance`)))
    (`/Engine/EditorBlueprintResources/StandardMacros.DoOnce` false :!label _label
      (:`Completed`
        (`GameplayStatics.PlaySoundAtLocation` "/Engine/EditorSounds/GamePreview/EndSimulate.EndSimulate" (`SceneComponent.K2_GetComponentLocation` _body) (struct) 3.0 1.5 0.0 null null null null)
        (`self.LaunchCharacter` (`self.TargetPlayer`) (`KismetMathLibrary.MakeVector` _returnvalue_x _returnvalue_y 300.0) false false)
        (bind (_direction _movement) (`Timeline|Timeline_0` :!via `PlayFromStart`)
          (:`Update`
            (bind (_returnvalue_x_2 _returnvalue_y_2 _returnvalue_z) (`KismetMathLibrary.BreakVector` (`KismetMathLibrary.Conv_DoubleToVector` _movement)))
            (`SceneComponent.SetWorldScale3D` (`self.Pivot`) (`KismetMathLibrary.MakeVector` 1.0 1.0 _returnvalue_z))
            (`SceneComponent.K2_AddWorldRotation` (`self.Pivot`) (struct :`Yaw` 4.0) false false)
            (`/Engine/EditorBlueprintResources/StandardMacros.DoOnce` false :!label _label_2
              (:`Completed`
                (`KismetSystemLibrary.Delay` 0.2)
                (`GameplayStatics.ApplyDamage` (`self.TargetPlayer`) 20.0 null self)
                (`KismetSystemLibrary.Delay` 2.0)
                (`self.ResetDoOnce`)
                (`self.Reset2`)
                (set `self.OrbitSide` (`KismetMathLibrary.RandomFloatInRange` -1.0 1.0))))))))))

(event `Reset2`
  ; Attack Player
  (goto _label_2 :!via `Reset`))

(event `ResetDoOnce`
  ; Attack Player
  (goto _label :!via `Reset`))

(event `self.ReceiveTick`
  (params (DeltaSeconds :type "Float (single-precision)"))
  (bind _targetplayer (`self.TargetPlayer`))
  ; Moving Towards and Around Player
  (`/Engine/EditorBlueprintResources/StandardMacros.IsValid` _targetplayer
    (:`Is Valid`
      (if (`self.IsDetected?`)
        (if (>= (`self.GetDistanceTo` _targetplayer) (`self.StoppingDistance`))
          (`|AIMoveTo` self (+ (`self.K2_GetActorLocation` (`self.TargetPlayer`)) (* (* (`self.OrbitSide`) (`SceneComponent.GetRightVector` (`/Game/Bridegroom/Blueprints/Player/PlayerCharacter_BP.Head` (`self.TargetPlayer`)))) 600.0)) null 30.0)
          (else
            (`MovementComponent.StopMovementImmediately` (`self.CharacterMovement`) :!label _label_3)))
        (else
          (goto _label_3))))))

(fn `UserConstructionScript`)