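; BP_ObjectivePoint is a quest trigger volume that shows an objective when the player walks into it.
; It creates an Instructions widget on BeginPlay, and the Construction Script sizes the overlap box from ObjectiveBoxSize.
; The first player overlap displays the title and content with a timed ObjFade, then sets ObjectiveInProgress.
; The CompletedObjective event replays the fade with a completion title but is not called within this Blueprint.
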(event `self.ReceiveBeginPlay`
  ; Begin Play
  (bind _returnvalue (`|CreateWidget` "/Game/Lee/QuestSystem/Blueprint/Instructions.Instructions_C" null (`self.Objective Title Text`) (`self.Objective Content Text`)))
  (set `self.Instructions` _returnvalue))

(event `self.ObjectiveBox.OnComponentBeginOverlap`
  (params (OverlappedComponent :type "PrimitiveComponent Object Reference") (OtherActor :type "Actor Object Reference") (OtherComp :type "PrimitiveComponent Object Reference") (OtherBodyIndex :type Integer) (bFromSweep :type Boolean) (SweepResult :type "HitResult Structure (by ref)"))
  (bind _instructions (`self.Instructions`))
  (bind _instructions_2 (`self.Instructions`))
  (bind _objfade (`/Game/Lee/QuestSystem/Blueprint/Instructions.ObjFade` _instructions_2))
  ; ObjectiveBox
  (if (== OtherActor (`GameplayStatics.GetPlayerCharacter` 0))
    (`/Engine/EditorBlueprintResources/StandardMacros.DoOnce` false
      (:`Completed`
        (set `/Game/Lee/QuestSystem/Blueprint/Instructions.ObjectiveTitleText` (`self.Objective Title Text`) _instructions)
        (set `/Game/Lee/QuestSystem/Blueprint/Instructions.ObjectiveContentText` (`self.Objective Content Text`) _instructions)
        (`UserWidget.AddToViewport` _instructions_2 0)
        (`UserWidget.PlayAnimation` _instructions_2 _objfade 0.0 1 "Forward" 1.0 false)
        (`KismetSystemLibrary.Delay` 5.0)
        (`UserWidget.PlayAnimation` _instructions_2 _objfade 0.0 1 "Reverse" 1.0 false)
        (set `self.ObjectiveInProgress?` true)))))

(event `CompletedObjective`
  (bind _instructions (`self.Instructions`))
  (bind _objfade (`/Game/Lee/QuestSystem/Blueprint/Instructions.ObjFade` _instructions))
  ; Completed Objective
  (set `/Game/Lee/QuestSystem/Blueprint/Instructions.ObjectiveTitleText` "Completed Objective" (`self.Instructions`))
  (`UserWidget.PlayAnimation` _instructions _objfade 0.0 1 "Forward" 1.0 false)
  (`KismetSystemLibrary.Delay` 3.0)
  (`UserWidget.PlayAnimation` _instructions _objfade 0.0 1 "Reverse" 1.0 false))

(fn `UserConstructionScript`
  (`BoxComponent.SetBoxExtent` (`self.ObjectiveBox`) (`self.Objective Box Size`) true))